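; BP_DoorObject is a door actor that swings open and closed through its UnlockDoor event.
; It stores its starting rotation at BeginPlay.
; UnlockDoor flips the DoorStatus flag and plays or reverses the DoorRotation timeline, with no key or lock check.
; Each timeline update combines the stored rotation with the animated yaw and sets it as the actor's relative rotation.
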(event EventUnlockDoor
  (if (Variables|Default|GetDoorStatus)
    (Variables|Default|SetDoorStatus false)
    (bind _doorrot (Timeline|DoorRotation Play)
      (:Update
        (Transformation|SetActorRelativeRotation (Math|Rotator|CombineRotators (Variables|Default|GetBeginRot) (Math|Rotator|MakeRotator 0.0 0.0 _doorrot)))))
    (else
      (Variables|Default|SetDoorStatus true)
      (Timeline|DoorRotation Reverse))))

(event EventBeginPlay
  (Variables|Default|SetBeginRot (Transformation|GetActorRotation)))

(event EventActorBeginOverlap
  (params (OtherActor :type Actor%20Object%20Reference)))

(event EventTick
  (params (DeltaSeconds :type Float%20%28single-precision%29)))

(fn ConstructionScript)