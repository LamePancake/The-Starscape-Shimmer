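; BP_ConsoleLeverInteract is a console lever that toggles between two positions each time PullConsoleLever is called.
; BeginPlay stores the actor's starting rotation as the base orientation.
; Each pull flips LeverStatus and plays or reverses the ConsoleLeverRotation timeline, whose output is combined as pitch with that base to rotate the whole actor.
; The file only animates the lever and triggers nothing else.
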(event EventPullConsoleLever
  (if (Variables|Default|GetLeverStatus)
    (Variables|Default|SetLeverStatus false)
    (bind _genrot (Timeline|Console%20Lever%20Rotation Play)
      (:Update
        (Transformation|SetActorRelativeRotation (Math|Rotator|CombineRotators (Variables|Default|GetLeverRotation) (Math|Rotator|MakeRotator 0.0 _genrot 0.0)))))
    (else
      (Variables|Default|SetLeverStatus true)
      (Timeline|Console%20Lever%20Rotation Reverse))))

(event EventBeginPlay
  (Variables|Default|SetLeverRotation (Transformation|GetActorRotation)))

(event EventActorBeginOverlap
  (params (OtherActor :type Actor%20Object%20Reference)))

(event EventTick
  (params (DeltaSeconds :type Float%20%28single-precision%29)))

(fn ConstructionScript)