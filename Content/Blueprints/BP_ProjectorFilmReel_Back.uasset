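; Back film reel actor for a projector that spins while switched on.
; It records its starting rotation on BeginPlay, and RunReel toggles whether it runs.
; While running, Tick restarts the ReelRot timeline each time it finishes, adding its roll to the starting rotation as the relative rotation.
; Switching off lets the current timeline cycle play out before the reel stops.
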(event EventBeginPlay
  (Variables|Default|SetBeginRot (Transformation|GetActorRotation)))

(event Collision|EventActorBeginOverlap
  (params (OtherActor :type Actor%20Object%20Reference)))

(event EventTick
  (params (DeltaSeconds :type Float%20%28single-precision%29))
  (if (Variables|Default|GetShouldRun)
    (if (not (Variables|Default|GetIsRunning))
      (Variables|Default|SetIsRunning true)
      (bind _reelrot (Timeline|ReelRot PlayFromStart)
        (:Update
          (Transformation|SetActorRelativeRotation (Math|Rotator|CombineRotators (Variables|Default|GetBeginRot) (Math|Rotator|MakeRotator _reelrot 0.0 0.0))))
        (:Finished
          (Variables|Default|SetIsRunning false))))))

(event EventRunReel
  (if (Variables|Default|GetShouldRun)
    (Variables|Default|SetShouldRun false)
    (else
      (Variables|Default|SetShouldRun true))))

(fn ConstructionScript)