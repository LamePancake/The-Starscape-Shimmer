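; BP_PosterObjective is an objective that is met when the poster film reel is in the projector.
; IsComplete finds the first BP_ProjectorInteract in the level and checks that its current film reel is valid and has "PosterFilm" as its first tag.
; OnComplete then sets the first BP_PosterPickup found in the level active.
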(event EventOnComplete
  (bind _outactors (Actor|GetAllActorsOfClass "/Game/Blueprints/BP_PosterPickup.BP_PosterPickup_C"))
  (Variables|/Script/TheStarscapeShimmer.InteractableObject|SetbIsActive (Utilities|Array|Get(acopy) _outactors) true))

(fn ConstructionScript)

(fn IsComplete
  (bind _outactors (Actor|GetAllActorsOfClass "/Game/Blueprints/BP_ProjectorInteract.BP_ProjectorInteract_C"))
  (if (!= (Variables|/Script/TheStarscapeShimmer.ProjectorInteract|GetCurrentFilmReel (Utilities|Array|Get(acopy) _outactors)) 0)
    (return (Utilities|Name|Equal(Name) (Utilities|Array|Get(acopy) (Variables|/Script/Engine.Actor|GetTags (Variables|/Script/TheStarscapeShimmer.ProjectorInteract|GetCurrentFilmReel (Utilities|Array|Get(acopy) _outactors)))) "PosterFilm"))
    (else
      (return false))))