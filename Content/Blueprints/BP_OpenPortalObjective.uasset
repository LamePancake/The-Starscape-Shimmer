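; Objective that opens a portal, judging by its name, once the final film reel is in the projector.
; IsComplete checks whether the first BP_ProjectorInteract in the level holds a film reel whose first tag is "FinalFilm".
; OnComplete searches for the TriggerSphere with that same first tag and turns on overlap events on its sphere component, arming the trigger.
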(event EventOnComplete
  (bind _outactors (Actor|GetAllActorsOfClass "/Script/Engine.TriggerSphere"))
  (bind _array_element (Utilities|Array|ForEachLoopwithBreak _outactors :!label _label)
    (:LoopBody
      (if (> (Utilities|Array|Length (Variables|/Script/Engine.Actor|GetTags _array_element)) 0)
        (if (Utilities|Name|Equal(Name) (Utilities|Array|Get(acopy) (Variables|/Script/Engine.Actor|GetTags _array_element)) "FinalFilm")
          (goto _label Break))))
    (:Completed
      (Variables|/Script/Engine.PrimitiveComponent|SetbGenerateOverlapEvents (Utilities|Array|Get(acopy) (Actor|GetComponentsByClass _array_element "/Script/Engine.SphereComponent")) true))))

(fn ConstructionScript)

(fn IsComplete
  (bind _outactors (Actor|GetAllActorsOfClass "/Game/Blueprints/BP_ProjectorInteract.BP_ProjectorInteract_C"))
  (if (!= (Variables|/Script/TheStarscapeShimmer.ProjectorInteract|GetCurrentFilmReel (Utilities|Array|Get(acopy) _outactors)) 0)
    (return (Utilities|Name|Equal(Name) (Utilities|Array|Get(acopy) (Variables|/Script/Engine.Actor|GetTags (Variables|/Script/TheStarscapeShimmer.ProjectorInteract|GetCurrentFilmReel (Utilities|Array|Get(acopy) _outactors)))) "FinalFilm"))
    (else
      (return false))))