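; BP_ReadFinalNoteObjective is an objective for reading a note, named as the final one.
; IsComplete reports whether the first RunNotePickup found in the level has been read.
; OnComplete searches the level's Emitter actors for one whose particle component has "NoteSpawner" as its first tag, then activates that particle system.
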(event EventOnComplete
  (bind _outactors (Actor|GetAllActorsOfClass "/Script/Engine.Emitter"))
  (bind _array_element (Utilities|Array|ForEachLoopwithBreak _outactors :!label _label)
    (:LoopBody
      (if (Utilities|Name|Equal(Name) (Utilities|Array|Get(acopy) (Variables|/Script/Engine.ActorComponent|GetComponentTags (Variables|/Script/Engine.Emitter|GetParticleSystemComponent _array_element))) "NoteSpawner")
        (goto _label Break)))
    (:Completed
      (Components|Activation|Activate (Variables|/Script/Engine.Emitter|GetParticleSystemComponent _array_element) false))))

(fn ConstructionScript)

(fn IsComplete
  (bind _outactors (Actor|GetAllActorsOfClass "/Script/TheStarscapeShimmer.RunNotePickup"))
  (bind _returnvalue (Class|RunNotePickup|RunNoteWasRead (Utilities|Array|Get(acopy) _outactors)))
  (return _returnvalue))