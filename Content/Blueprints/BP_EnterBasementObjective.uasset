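; BP_EnterBasementObjective is an objective that checks the state of the basement door to decide whether it is complete.
; IsComplete scans every BP_DoorObject for one whose first tag is "BasementDoor" and returns the inverse of its DoorStatus.
; With no tagged match, the check falls through to whatever element the loop last held.
; OnActivate and OnComplete only print test messages.
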(event EventOnActivate
  (Development|PrintString "Activated Test Objective"))

(event EventOnComplete
  (Development|PrintString "Completed Test Objective"))

(fn ConstructionScript)

(fn IsComplete
  (bind _outactors (Actor|GetAllActorsOfClass "/Game/Blueprints/BP_DoorObject.BP_DoorObject_C"))
  (bind _array_element (Utilities|Array|ForEachLoopwithBreak _outactors :!label _label)
    (:LoopBody
      (if (> (Utilities|Array|Length (Variables|/Script/Engine.Actor|GetTags _array_element)) 0)
        (if (Utilities|Name|Equal(Name) (Utilities|Array|Get(acopy) (Variables|/Script/Engine.Actor|GetTags _array_element)) "BasementDoor")
          (goto _label Break))))
    (:Completed
      (return (not (Variables|/Game/Blueprints/BP_DoorObject.BP_DoorObject_C|GetDoorStatus _array_element))))))