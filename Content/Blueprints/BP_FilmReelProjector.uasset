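; BP_FilmReelProjector is a film reel actor that shows and spins its static mesh while ShouldRun is set, and hides it otherwise.
; Tick polls ShouldRun and restarts the ReelRot timeline whenever IsRunning is clear, so the spin repeats.
; The timeline applies its value as roll combined with the rotation saved at BeginPlay.
; Clearing ShouldRun hides the mesh but leaves the current timeline pass to finish.
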(event EventBeginPlay
  (Variables|Default|SetBeginRot (Transformation|GetActorRotation)))

(event EventActorBeginOverlap
  (params (OtherActor :type Actor%20Object%20Reference)))

(event EventTick
  (params (DeltaSeconds :type Float%20%28single-precision%29))
  (if (Variables|Default|GetShouldRun)
    (Rendering|SetVisibility (Variables|Default|GetStaticMesh) true true)
    (if (not (Variables|Default|GetIsRunning))
      (Variables|Default|SetIsRunning true)
      (bind _reelrot (Timeline|ReelRot PlayFromStart)
        (:Update
          (Transformation|SetActorRelativeRotation (Math|Rotator|CombineRotators (Variables|Default|GetBeginRot) (Math|Rotator|MakeRotator _reelrot 0.0 0.0))))
        (:Finished
          (Variables|Default|SetIsRunning false))))
    (else
      (Rendering|SetVisibility (Variables|Default|GetStaticMesh) false true))))

(fn ConstructionScript)