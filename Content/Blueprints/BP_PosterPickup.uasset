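; BP_PosterPickup is a poster pickup that has gravity enabled on its mesh the first time the player interacts with it.
; On interaction, a helper checks the active and first-interaction flags, clears the latter, and turns on gravity for the first static mesh component.
; When that succeeds, it calls Grip on the first-person character.
; A pick-up event also clears the first-interaction flag, so later interactions skip this step.
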(event EventOnInteraction
  (params (Character :type First%20Person%20Character%20Object%20Reference))
  (bind _addedgravity (CallFunction|AddGravityonFirstInteraction))
  (if _addedgravity
    (bind _asbp_first_person_character (Utilities|Casting|CastToBP_FirstPersonCharacter (Game|GetPlayerCharacter 0))
      (:then
        (Class|FirstPersonCharacter|Grip _asbp_first_person_character))
      (:CastFailed
        (Development|PrintString ":(")))))

(event EventOnPickUp
  (Variables|Default|SetIsFirstInteraction false))

(fn ConstructionScript)

(fn AddGravityonFirstInteraction
  (if (Variables|Default|GetbIsActive)
    (if (Variables|Default|GetIsFirstInteraction)
      (Variables|Default|SetIsFirstInteraction false)
      (Physics|SetEnableGravity (Utilities|Array|Get(acopy) (Actor|GetComponentsByClass "/Script/Engine.StaticMeshComponent")) true)
      (return true)
      (else
        (return false)))
    (else
      (return false))))