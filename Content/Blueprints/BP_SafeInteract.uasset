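; BP_SafeInteract is an interactable safe actor that swings open or closed through its UnlockSafe event.
; BeginPlay stores the actor's starting rotation.
; Each UnlockSafe call flips SafeStatus and either plays or reverses the SafeRotation timeline.
; The timeline's SafeRot track drives a yaw offset, combined with the starting rotation and applied as the actor's relative rotation.
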(event EventUnlockSafe
  (if (Variables|Default|GetSafeStatus)
    (Variables|Default|SetSafeStatus false)
    (bind _saferot (Timeline|SafeRotation Play)
      (:Update
        (Transformation|SetActorRelativeRotation (Math|Rotator|CombineRotators (Variables|Default|GetBeginRot) (Math|Rotator|MakeRotator 0.0 0.0 _saferot)))))
    (else
      (Variables|Default|SetSafeStatus true)
      (Timeline|SafeRotation Reverse))))

(event EventBeginPlay
  (Variables|Default|SetBeginRot (Transformation|GetActorRotation)))

(event EventActorBeginOverlap
  (params (OtherActor :type Actor%20Object%20Reference)))

(event EventTick
  (params (DeltaSeconds :type Float%20%28single-precision%29)))

(fn ConstructionScript)