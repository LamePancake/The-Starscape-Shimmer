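; Interactable generator actor that toggles its GeneratorStatus flag and animates its rotation when PullLever is called.
; BeginPlay caches the starting rotation, and each pull plays or reverses the GeneratorRotation timeline based on the flag, clearing it on play and setting it on reverse.
; The timeline's GenRot track supplies a pitch offset that is combined with the cached rotation and applied as the actor's relative rotation.
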(event EventBeginPlay
  (Variables|Default|SetBeginGenRot (Transformation|GetActorRotation)))

(event EventActorBeginOverlap
  (params (OtherActor :type Actor%20Object%20Reference)))

(event EventTick
  (params (DeltaSeconds :type Float%20%28single-precision%29)))

(event EventPullLever
  (if (Variables|Default|GetGeneratorStatus)
    (Variables|Default|SetGeneratorStatus false)
    (bind _genrot (Timeline|Generator%20Rotation Play)
      (:Update
        (Transformation|SetActorRelativeRotation (Math|Rotator|CombineRotators (Variables|Default|GetBeginGenRot) (Math|Rotator|MakeRotator 0.0 _genrot 0.0)))))
    (else
      (Variables|Default|SetGeneratorStatus true)
      (Timeline|Generator%20Rotation Reverse))))

(fn ConstructionScript)